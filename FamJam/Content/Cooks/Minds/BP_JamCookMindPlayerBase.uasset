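; Base player-driven cook mind that turns a local player's input into trigger impulses.
; SetController has the PlayerId's controller possess it, adds the trigger Enhanced Input mapping context and points the view at the first CameraActor found, then runs the parent's setup.
; Ten trigger input actions each call AddImpulse with their trigger number and HitStart on Started; releases are not handled here.
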(event Input|EnhancedActionEvents|EnhancedInputActionIA_Trigger1
  (params (ActionValue :type Boolean) (ElapsedSeconds :type Float%20%28double-precision%29) (TriggeredSeconds :type Float%20%28double-precision%29) (InputAction :type Input%20Action%20Object%20Reference :default "/Game/Cooks/Minds/Triggers/Player/IA_Trigger1.IA_Trigger1"))
  (:Started
    (CallFunction|AddImpulse 1 "HitStart")))

(event Input|EnhancedActionEvents|EnhancedInputActionIA_Trigger2
  (params (ActionValue :type Boolean) (ElapsedSeconds :type Float%20%28double-precision%29) (TriggeredSeconds :type Float%20%28double-precision%29) (InputAction :type Input%20Action%20Object%20Reference :default "/Game/Cooks/Minds/Triggers/Player/IA_Trigger2.IA_Trigger2"))
  (:Started
    (CallFunction|AddImpulse 2 "HitStart")))

(event Input|EnhancedActionEvents|EnhancedInputActionIA_Trigger3
  (params (ActionValue :type Boolean) (ElapsedSeconds :type Float%20%28double-precision%29) (TriggeredSeconds :type Float%20%28double-precision%29) (InputAction :type Input%20Action%20Object%20Reference :default "/Game/Cooks/Minds/Triggers/Player/IA_Trigger3.IA_Trigger3"))
  (:Started
    (CallFunction|AddImpulse 3 "HitStart")))

(event Input|EnhancedActionEvents|EnhancedInputActionIA_Trigger4
  (params (ActionValue :type Boolean) (ElapsedSeconds :type Float%20%28double-precision%29) (TriggeredSeconds :type Float%20%28double-precision%29) (InputAction :type Input%20Action%20Object%20Reference :default "/Game/Cooks/Minds/Triggers/Player/IA_Trigger4.IA_Trigger4"))
  (:Started
    (CallFunction|AddImpulse 4 "HitStart")))

(event Input|EnhancedActionEvents|EnhancedInputActionIA_Trigger5
  (params (ActionValue :type Boolean) (ElapsedSeconds :type Float%20%28double-precision%29) (TriggeredSeconds :type Float%20%28double-precision%29) (InputAction :type Input%20Action%20Object%20Reference :default "/Game/Cooks/Minds/Triggers/Player/IA_Trigger5.IA_Trigger5"))
  (:Started
    (CallFunction|AddImpulse 5 "HitStart")))

(event Input|EnhancedActionEvents|EnhancedInputActionIA_Trigger6
  (params (ActionValue :type Boolean) (ElapsedSeconds :type Float%20%28double-precision%29) (TriggeredSeconds :type Float%20%28double-precision%29) (InputAction :type Input%20Action%20Object%20Reference :default "/Game/Cooks/Minds/Triggers/Player/IA_Trigger6.IA_Trigger6"))
  (:Started
    (CallFunction|AddImpulse 6 "HitStart")))

(event Input|EnhancedActionEvents|EnhancedInputActionIA_Trigger7
  (params (ActionValue :type Float%20%28double-precision%29) (ElapsedSeconds :type Float%20%28double-precision%29) (TriggeredSeconds :type Float%20%28double-precision%29) (InputAction :type Input%20Action%20Object%20Reference :default "/Game/Cooks/Minds/Triggers/Player/IA_Trigger7.IA_Trigger7"))
  (:Started
    (CallFunction|AddImpulse 7 "HitStart")))

(event Input|EnhancedActionEvents|EnhancedInputActionIA_Trigger8
  (params (ActionValue :type Float%20%28double-precision%29) (ElapsedSeconds :type Float%20%28double-precision%29) (TriggeredSeconds :type Float%20%28double-precision%29) (InputAction :type Input%20Action%20Object%20Reference :default "/Game/Cooks/Minds/Triggers/Player/IA_Trigger8.IA_Trigger8"))
  (:Started
    (CallFunction|AddImpulse 8 "HitStart")))

(event Input|EnhancedActionEvents|EnhancedInputActionIA_Trigger9
  (params (ActionValue :type Boolean) (ElapsedSeconds :type Float%20%28double-precision%29) (TriggeredSeconds :type Float%20%28double-precision%29) (InputAction :type Input%20Action%20Object%20Reference :default "/Game/Cooks/Minds/Triggers/Player/IA_Trigger9.IA_Trigger9"))
  (:Started
    (CallFunction|AddImpulse 9 "HitStart")))

(event Input|EnhancedActionEvents|EnhancedInputActionIA_Trigger10
  (params (ActionValue :type Boolean) (ElapsedSeconds :type Float%20%28double-precision%29) (TriggeredSeconds :type Float%20%28double-precision%29) (InputAction :type Input%20Action%20Object%20Reference :default "/Game/Cooks/Minds/Triggers/Player/IA_Trigger10.IA_Trigger10"))
  (:Started
    (CallFunction|AddImpulse 10 "HitStart")))

(event EventBeginPlay
  (|CallParentFunction))

(event Collision|EventActorBeginOverlap
  (params (OtherActor :type Actor%20Object%20Reference))
  (|CallParentFunction OtherActor) ; This node is disabled and will not be called.\nDrag off pins to build functionality.
)

(event EventTick
  (params (DeltaSeconds :type Float%20%28single-precision%29))
  (|CallParentFunction DeltaSeconds) ; This node is disabled and will not be called.\nDrag off pins to build functionality.
)

(fn ConstructionScript
  (|CallParentFunction))

(fn SetController
  (bind _playerid (Variables|Default|GetPlayerId))
  (bind _returnvalue (Game|GetPlayerController _playerid))
  (Pawn|Possess _returnvalue self)
  (Input|AddMappingContext (PlayerController|LocalPlayerSubsystems|GetEnhancedInputLocalPlayerSubsystem _returnvalue) "/Game/Cooks/Minds/Triggers/Player/IMC_PlayerTrigger.IMC_PlayerTrigger" 0 "(bIgnoreAllPressedKeysUntilRelease=True,bForceImmediately=False,bNotifyUserSettings=False)")
  (bind _returnvalue_2 (Actor|GetActorOfClass "/Script/Engine.CameraActor"))
  (Game|Player|SetViewTargetwithBlend _returnvalue _returnvalue_2 0.0 "VTBlend_Linear" 0.0 false)
  (|CallParentFunction))