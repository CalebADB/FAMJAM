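; Base actor for a cook's "thought": a button prompt sprite timed to a musical measure in the cook thought visualizer.
; Setters supply button type (sprite, with error-sprite fallback), hit measure and ingress path.
; UpdateTime fades the sprite in and slides it along that path to its relative origin as the hit measure nears.
; BeginPlay runs a MiseEnPlace readiness check, though its failure assignment is unreachable.
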(event EventBeginPlay
  (CallFunction|MiseEnPlace))

(fn ConstructionScript)

(fn MiseEnPlace
  (Variables|Default|SetbMiseEnPlace true)
  (bind _enumvalue (|ForEachEJamCookThoughtVisualizerButtonType)
    (:LoopBody
      (if (.ReturnValue (Utilities|Map|Find (Variables|Default|GetButtonTypeToErrorSprite) _enumvalue))
        _))
    (:then
      (if (not (Variables|Default|GetbMiseEnPlace))
        (Development|PrintText (Utilities|Text|ToText(String) (Utilities|String|Append (Utilities|GetDisplayName self) ": Failed MiseEnPlace. Forgiving because Darius is Debugging")) true true "(R=1.000000,G=0.000000,B=0.000000,A=1.000000)" 1e+01)
        (Variables|Default|SetbMiseEnPlace true)))))

(fn SetButtonType
  (params (ButtonType :type EJamCookThoughtVisualizerButtonType%20Enum :default "PS"))
  (bind _rendercomponent (Variables|Default|GetRenderComponent))
  (if (Variables|Default|GetbMiseEnPlace)
    (bind _output_get (Variables|Default|SetButtonType ButtonType))
    (if (.ReturnValue (Utilities|Map|Find (Variables|Default|GetButtonTypeToSprite) _output_get))
      (Rendering|Components|Sprite|SetSprite _rendercomponent (.Value (Utilities|Map|Find (Variables|Default|GetButtonTypeToSprite) _output_get)))
      (else
        (Rendering|Components|Sprite|SetSprite _rendercomponent (.Value (Utilities|Map|Find (Variables|Default|GetButtonTypeToErrorSprite) _output_get)))))))

(fn SetIngressPath
  (params (IngressDirection :type Vector) (Speed :type Float%20%28double-precision%29))
  (Variables|Default|SetIngressPath (* IngressDirection Speed)))

(fn SetTiming
  (params (MeasureHit :type Float%20%28double-precision%29))
  (Variables|Default|SetMeasureHit MeasureHit))

(fn UpdateTime
  (params (CurrentMeasure :type Float%20%28double-precision%29))
  (bind _measurehit (Variables|Default|GetMeasureHit))
  (bind _measuredistancemax (Variables|Default|GetMeasureDistanceMax))
  (bind _returnvalue (- _measurehit CurrentMeasure))
  (bind _returnvalue_2 (Math|Float|Clamp(Float) _returnvalue 0.0 _measuredistancemax))
  (if (Variables|Default|GetbMiseEnPlace)
    (Sprite|SetSpriteColor (Variables|Default|GetRenderComponent) (Utilities|Struct|MakeLinearColor 1.0 1.0 1.0 (/ (- _measuredistancemax _returnvalue_2) _measuredistancemax)))
    (Transformation|SetActorRelativeLocation (* _returnvalue_2 (Variables|Default|GetIngressPath)))))