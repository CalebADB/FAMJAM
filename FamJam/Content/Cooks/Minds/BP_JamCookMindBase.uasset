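; BP_JamCookMindBase is a base Blueprint for jam cook minds, holding a map of trigger IDs to impulse lists.
; BeginPlay calls SetController, an empty hook here.
; AddImpulse acts only on existing triggers, re-adding the map entry with the impulse stored as an integer.
; It removes the entry before reading its impulses, so earlier impulses appear not to carry over.
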(event EventBeginPlay
  (CallFunction|SetController))

(event Collision|EventActorBeginOverlap
  (params (OtherActor :type Actor%20Object%20Reference)))

(event EventTick
  (params (DeltaSeconds :type Float%20%28single-precision%29)))

(fn ConstructionScript)

(fn SetController)

(fn AddImpulse
  (params (TriggerId :type Integer) (Impulse :type EJamCookImpulse%20Enum :default "HitStart"))
  (bind _triggers (Variables|Default|GetTriggers))
  (bind (_value _returnvalue) (Utilities|Map|Find _triggers TriggerId))
  (if _returnvalue
    (Utilities|Map|Remove _triggers TriggerId)
    (bind _output_get (LocalVariables|SetNewImpulses (Utilities|Struct|BreakJamCookTrigger _value)))
    (Utilities|Array|Add _output_get (Math|Conversions|ToInteger(Byte) Impulse))
    (Utilities|Map|Add _triggers TriggerId (Utilities|Struct|MakeJamCookTrigger (LocalVariables|GetNewImpulses)))))