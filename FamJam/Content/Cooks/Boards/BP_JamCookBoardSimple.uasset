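; BP_JamCookBoardSimple is a simple cook board Blueprint that extends a parent board's Scoop behavior.
; Scoop passes the incoming chunk's tempo and the requested tempo to the CaldronMouth component as the ChunkBPM and ChopBPM float parameters, then calls the parent implementation.
; All other logic comes from the parent, as the event stubs are disabled and the construction script only calls its parent.
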(event EventBeginPlay
  (|CallParentFunction) ; This node is disabled and will not be called.\nDrag off pins to build functionality.
)

(event Collision|EventActorBeginOverlap
  (params (OtherActor :type Actor%20Object%20Reference))
  (|CallParentFunction OtherActor) ; This node is disabled and will not be called.\nDrag off pins to build functionality.
)

(event EventTick
  (params (DeltaSeconds :type Float%20%28single-precision%29))
  (|CallParentFunction DeltaSeconds) ; This node is disabled and will not be called.\nDrag off pins to build functionality.
)

(fn ConstructionScript
  (|CallParentFunction))

(fn Scoop
  (params (StartTime :type Float%20%28double-precision%29) (Tempo :type Float%20%28double-precision%29) (Chunk :type Jam%20Chunk%20Structure))
  (bind _caldronmouth (Variables|Default|GetCaldronMouth))
  (Audio|Parameter|SetFloatParameter _caldronmouth "ChunkBPM" (.Tempo (Utilities|Struct|BreakJamChunk Chunk)) :!class /Script/Engine.AudioComponent)
  (Audio|Parameter|SetFloatParameter _caldronmouth "ChopBPM" Tempo :!class /Script/Engine.AudioComponent)
  (|CallParentFunction StartTime Tempo Chunk))