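; BP_Jam is an actor that displays the Chef's current recipe and its progress through a BP_JamRecipeVisualizer.
; Each tick it polls and clears a flag on the Chef, then replaces any existing visualizer with a newly spawned one attached to itself, initialized from the recipe and overview.
; While a visualizer exists, it receives the Chef's step index and remaining measures every tick.
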(event EventBeginPlay)

(event Collision|EventActorBeginOverlap
  (params (OtherActor :type Actor%20Object%20Reference)))

(event EventBlueprintTick
  (params (DeltaTime :type Float%20%28single-precision%29))
  (bind _chef (Variables|Default|GetChef))
  (if (Variables|/Script/FamJam.JamChef|GetbShouldInitializeJamVisualizer _chef)
    (Variables|/Script/FamJam.JamChef|SetbShouldInitializeJamVisualizer _chef false)
    (CallFunction|StartVisualizer))
  (if (not (== (Variables|Default|GetRecipeVisualizer) 0))
    (CallFunction|UpdateVisualizer)))

(fn ConstructionScript)

(fn StartVisualizer
  (bind _chef (Variables|Default|GetChef))
  (if (!= (Variables|Default|GetRecipeVisualizer) 0)
    (Actor|DestroyActor (Variables|Default|GetRecipeVisualizer)))
  (bind _returnvalue (Game|SpawnActorfromClass "/Game/Jam/Recipes/Visualizer/BP_JamRecipeVisualizer.BP_JamRecipeVisualizer_C" (Math|Transform|MakeTransform "0, 0, 0" "0, 0, 0" "1.000000,1.000000,1.000000") "Undefined" "MultiplyWithRoot" 0 0))
  (Transformation|AttachActorToActor _returnvalue self "None" "KeepRelative" "KeepRelative" "KeepRelative" true)
  (Variables|Default|SetRecipeVisualizer _returnvalue)
  (Default|Initialize _returnvalue (Variables|/Script/FamJam.JamChef|GetRecipeOverview _chef) (Variables|/Script/FamJam.JamChef|GetRecipe _chef)))

(fn UpdateVisualizer
  (bind _chef (Variables|Default|GetChef))
  (Default|Update (Variables|Default|GetRecipeVisualizer) (Variables|/Script/FamJam.JamChef|GetStepIdx _chef) (Variables|/Script/FamJam.JamChef|GetMeasureRemaining _chef)))