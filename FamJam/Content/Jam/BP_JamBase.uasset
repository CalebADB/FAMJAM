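; BP_JamBase is a base actor for jams that can display a recipe visualizer driven by Chef state.
; StartVisualizer replaces any existing BP_JamRecipeVisualizer, attaches a new one and initializes it with the Chef's recipe data.
; UpdateVisualizer passes it the current step and measures remaining until the next step.
; The flag-driven logic that calls both functions is disconnected; BeginPlay, overlap and Tick do nothing.
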(event EventBeginPlay)

(event Collision|EventActorBeginOverlap
  (params (OtherActor :type Actor%20Object%20Reference)))

(event EventBlueprintTick
  (params (DeltaTime :type Float%20%28single-precision%29)))

(fn ConstructionScript)

(fn StartVisualizer
  (bind _chef (Variables|Default|GetChef))
  (if (!= (Variables|Default|GetRecipeVisualizer) 0)
    (Actor|DestroyActor (Variables|Default|GetRecipeVisualizer)))
  (bind _returnvalue (Game|SpawnActorfromClass "/Game/Jam/Visualizer/BP_JamRecipeVisualizer.BP_JamRecipeVisualizer_C" (Math|Transform|MakeTransform "0, 0, 0" "0, 0, 0" "1.000000,1.000000,1.000000") "Undefined" "MultiplyWithRoot" 0 0))
  (Transformation|AttachActorToActor _returnvalue self "None" "KeepRelative" "KeepRelative" "KeepRelative" true)
  (Variables|Default|SetRecipeVisualizer _returnvalue)
  (Default|Initialize _returnvalue (Variables|/Script/FamJam.JamChef|GetRecipeOverview _chef) (Variables|/Script/FamJam.JamChef|GetRecipe _chef))
  (Variables|/Script/FamJam.JamChef|SetbIsVisualizingJam _chef true))

(fn UpdateVisualizer
  (bind _chef (Variables|Default|GetChef))
  (Default|Update (Variables|Default|GetRecipeVisualizer) (Variables|/Script/FamJam.JamChef|GetStepIdx _chef) (- (Variables|/Script/FamJam.JamChef|GetNextStepMeasureIdx _chef) (Variables|/Script/FamJam.JamChef|GetMeasureIdx _chef))))