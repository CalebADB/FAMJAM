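; Actor for a single tile in the Jam visualizer, switched between an on color and an off color.
; Initialize scales and offsets the Tile component from layer, width and height using LayerDepth, stores both colors and starts the tile off.
; SetColorOn pushes the chosen color into the "Color" vector parameter on the tile's materials.
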(event EventBeginPlay)

(event Collision|EventActorBeginOverlap
  (params (OtherActor :type Actor%20Object%20Reference)))

(event EventTick
  (params (DeltaSeconds :type Float%20%28single-precision%29)))

(fn ConstructionScript)

(fn Initialize
  (params (InLayer :type Float%20%28double-precision%29) (InWidth :type Float%20%28double-precision%29) (InHeight :type Float%20%28double-precision%29) (ColorOn :type Color%20Structure) (ColorOff :type Color%20Structure))
  (bind _tile (Variables|Default|GetTile))
  (Transformation|SetWorldScale3D _tile (Math|Vector|MakeVector (/ (Variables|Default|GetLayerDepth) 1e+02) (/ InWidth 1e+02) (/ InHeight 1e+02)))
  (Transformation|SetRelativeLocation _tile (Math|Vector|MakeVector (* InLayer (Variables|Default|GetLayerDepth)) (/ InWidth 2.0) (/ InHeight -2.0)) false false)
  (Variables|Default|SetTileColorOn ColorOn)
  (Variables|Default|SetTileColorOff ColorOff)
  (CallFunction|SetColoron false))

(fn SetColoron
  (params (On :type Boolean))
  (bind _tilecoloroff (Variables|Default|GetTileColorOff))
  (bind _tilecoloron (Variables|Default|GetTileColorOn))
  (bind _tile (Variables|Default|GetTile))
  (bind _returnvalue (Math|Conversions|ToLinearColor(Color) _tilecoloroff))
  (bind _returnvalue_2 (Math|Conversions|ToLinearColor(Color) _tilecoloron))
  (bind (_r _g _b) (Utilities|Struct|BreakLinearColor _returnvalue_2))
  (bind (_r_2 _g_2 _b_2) (Utilities|Struct|BreakLinearColor _returnvalue))
  (if On
    (Rendering|Material|SetVectorParameterValueonMaterials _tile "Color" (Math|Vector|MakeVector _r _g _b))
    (else
      (Rendering|Material|SetVectorParameterValueonMaterials _tile "Color" (Math|Vector|MakeVector _r_2 _g_2 _b_2)))))