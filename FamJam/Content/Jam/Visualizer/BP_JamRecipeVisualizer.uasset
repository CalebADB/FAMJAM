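; BP_JamRecipeVisualizer builds a timeline view of a Jam recipe from spawned, attached actors.
; Initialize lays out colored cook rows with alternating-color layers, measure dividers and a playhead, then places chop visualizers on their layers with step dividers.
; Update moves the playhead from step index and remaining measures, while UpdateTiles is still an empty stub.
; On destruction it loops to destroy its attached actors.
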(event EventBeginPlay)

(event Collision|EventActorBeginOverlap
  (params (OtherActor :type Actor%20Object%20Reference)))

(event EventTick
  (params (DeltaSeconds :type Float%20%28single-precision%29)))

(event EventDestroyed
  (bind _self self)
  (bind _outactors (Actor|GetAttachedActors _self true false))
  (if (not (== (Utilities|Array|Length _outactors) 0)) :!label _label
    (Actor|DestroyActor (Utilities|Array|Get(acopy) _outactors))
    (goto _label)))

(fn ConstructionScript)

(fn Initialize
  (params (RecipeOverview :type Jam%20Recipe%20Overview%20Structure) (Recipe :type Jam%20Recipe%20Object%20Reference))
  (bind _output_get (Variables|Default|SetRecipeOverview RecipeOverview))
  (if (!= (Utilities|Map|Length (.CookNameToOverviewMap (Utilities|Struct|BreakJamRecipeOverview _output_get))) 0)
    (Variables|Default|SetRecipe Recipe)
    (CallFunction|AddTable)
    (CallFunction|AddSteps)
    (else
      (Development|PrintText "Overview is missing Cooks. Recipe is being thrown" true true "(R=1.000000,G=0.000000,B=0.026946,A=1.000000)" 2e+01))))

(fn AddTable
  (bind _cookvisualizers (Variables|Default|GetCookVisualizers))
  (bind _measureverticallength (Variables|Default|GetMeasureVerticalLength))
  (bind _measureverticalspacing (Variables|Default|GetMeasureVerticalSpacing))
  (bind _recipeoverview (Variables|Default|GetRecipeOverview))
  (bind _measurehorizontalspacing (Variables|Default|GetMeasureHorizontalSpacing))
  (bind _measurehorizontallength (Variables|Default|GetMeasureHorizontalLength))
  (bind _returnvalue (Math|Float|Floor (.lastmeasure _recipeoverview)))
  (bind _returnvalue_2 (+ _measureverticallength _measureverticalspacing))
  (bind _returnvalue_3 (* (.lastmeasure _recipeoverview) _measurehorizontallength))
  (bind _returnvalue_4 (* _returnvalue _measurehorizontalspacing))
  (bind _returnvalue_5 (+ _returnvalue_3 _returnvalue_4))
  (Variables|Default|SetCookSpawnVerticalPosition (/ (Variables|Default|GetCookVerticalSpacing) -2.0))
  (bind _keys (Utilities|Map|Keys (.cooknametooverviewmap _recipeoverview)))
  (for _array_element _keys
    (bind _returnvalue_6 (Game|SpawnActorfromClass "/Game/Jam/Visualizer/BP_JamCookVisualizer.BP_JamCookVisualizer_C" (Math|Transform|MakeTransform (Math|Vector|MakeVector 0.0 0.0 (Variables|Default|GetCookSpawnVerticalPosition)) "0, 0, 0" "1.000000,1.000000,1.000000") "Undefined" "MultiplyWithRoot" 0 0))
    (Transformation|AttachActorToActor _returnvalue_6 self "None" "KeepRelative" "KeepRelative" "KeepRelative" true)
    (Utilities|Map|Add _cookvisualizers _array_element (Utilities|Struct|MakeF_JamCookVisualizerContainer _returnvalue_6))
    (Default|Initialize :self _returnvalue_6 :InLayer 3.0 :InWidth _returnvalue_5 :InHeight (* (+ (Variables|Default|GetCookLayerVerticalSpacing) (Variables|Default|GetMeasureVerticalLength) (Variables|Default|GetMeasureVerticalSpacing)) (Utilities|Array|Length (.BoardClasses (Utilities|Struct|BreakJamRecipeCookOverview (.Value (Utilities|Map|Find (.cooknametooverviewmap _recipeoverview) _array_element)))))) :ColorOff (.CookColor (Utilities|Struct|BreakJamRecipeCookOverview (.Value (Utilities|Map|Find (.cooknametooverviewmap _recipeoverview) _array_element)))))
    (Variables|Default|SetCookLayerSpawnVerticalPosition (/ (Variables|Default|GetCookLayerVerticalSpacing) -2.0))
    (for _index (range 1 (Utilities|Array|Length (.BoardClasses (Utilities|Struct|BreakJamRecipeCookOverview (.Value (Utilities|Map|Find (.cooknametooverviewmap _recipeoverview) _array_element))))))
      (bind _returnvalue_7 (Game|SpawnActorfromClass "/Game/Jam/Visualizer/BP_JamCookLayerVisualizer.BP_JamCookLayerVisualizer_C" (Math|Transform|MakeTransform (Math|Vector|MakeVector 0.0 0.0 (Variables|Default|GetCookLayerSpawnVerticalPosition)) "0, 0, 0" "1.000000,1.000000,1.000000") "Undefined" "MultiplyWithRoot" 0 0))
      (Transformation|AttachActorToActor _returnvalue_7 (.CookVisualizer (Utilities|Struct|BreakF_JamCookVisualizerContainer (.Value (Utilities|Map|Find _cookvisualizers _array_element)))) "None" "KeepRelative" "KeepRelative" "KeepRelative" true)
      (Utilities|Array|Add (LocalVariables|GetCookLayerVisualizers) (Utilities|Struct|MakeF_JamCookLayerVisualizerContainer _returnvalue_7))
      (if (LocalVariables|GetShouldUseCookLayerColorA)
        (Default|Initialize :self _returnvalue_7 :InLayer 2.0 :InWidth _returnvalue_5 :InHeight _returnvalue_2 :ColorOff (LocalVariables|GetCookLayerColorA))
        (LocalVariables|SetShouldUseCookLayerColorA false)
        (else
          (Default|Initialize :self _returnvalue_7 :InLayer 2.0 :InWidth _returnvalue_5 :InHeight _returnvalue_2 :ColorOff (LocalVariables|GetCookLayerColorB))
          (LocalVariables|SetShouldUseCookLayerColorA true)))
      (Variables|Default|SetCookLayerSpawnVerticalPosition (- (- (Variables|Default|GetCookLayerSpawnVerticalPosition) (+ (Variables|Default|GetMeasureVerticalLength) (Variables|Default|GetMeasureVerticalSpacing))) (Variables|Default|GetCookLayerVerticalSpacing))))
    (Variables|Default|SetCookSpawnVerticalPosition (- (- (Variables|Default|GetCookSpawnVerticalPosition) (* (+ (Variables|Default|GetCookLayerVerticalSpacing) (Variables|Default|GetMeasureVerticalLength) (Variables|Default|GetMeasureVerticalSpacing)) (Utilities|Array|Length (.BoardClasses (Utilities|Struct|BreakJamRecipeCookOverview (.Value (Utilities|Map|Find (.cooknametooverviewmap _recipeoverview) _array_element))))))) (Variables|Default|GetCookVerticalSpacing)))
    (bind _output_get (LocalVariables|SetCookVisualizer (.CookVisualizer (Utilities|Struct|BreakF_JamCookVisualizerContainer (.Value (Utilities|Map|Find _cookvisualizers _array_element))))))
    (Utilities|Map|Remove _cookvisualizers _array_element)
    (Utilities|Map|Add _cookvisualizers _array_element (Utilities|Struct|MakeF_JamCookVisualizerContainer _output_get (LocalVariables|GetCookLayerVisualizers)))
    (Utilities|Array|Clear (LocalVariables|GetCookLayerVisualizers)))
  (Variables|Default|SetCookSpawnVerticalPosition (- (Variables|Default|GetCookSpawnVerticalPosition) (/ (Variables|Default|GetCookVerticalSpacing) -2.0)))
  (for _index_2 (range 1 (Math|Float|Floor (.lastmeasure _recipeoverview)))
    (bind _returnvalue_8 (Game|SpawnActorfromClass "/Game/Jam/Visualizer/BP_JamRecipeDivider.BP_JamRecipeDivider_C" (Math|Transform|MakeTransform (Math|Vector|MakeVector 0.0 (+ (* _index_2 (Variables|Default|GetMeasureHorizontalLength)) (* (- _index_2 1.0) (Variables|Default|GetMeasureHorizontalSpacing))) 0.0) "0, 0, 0" "1.000000,1.000000,1.000000") "Undefined" "MultiplyWithRoot" 0 0))
    (Transformation|AttachActorToActor _returnvalue_8 self "None" "KeepRelative" "KeepRelative" "KeepRelative" true)
    (Default|Initialize :self _returnvalue_8 :InLayer 1.75 :InWidth (Variables|Default|GetMeasureHorizontalSpacing) :InHeight (* (Variables|Default|GetCookSpawnVerticalPosition) -1.0) :ColorOff (LocalVariables|GetMeasureDividerColor)))
  (bind _returnvalue_9 (Game|SpawnActorfromClass "/Game/Jam/Visualizer/BP_JamRecipePlayhead.BP_JamRecipePlayhead_C" (Math|Transform|MakeTransform "0, 0, 0" "0, 0, 0" "1.000000,1.000000,1.000000") "Undefined" "MultiplyWithRoot" 0 0))
  (Transformation|AttachActorToActor _returnvalue_9 self "None" "KeepRelative" "KeepRelative" "KeepRelative" true)
  (Default|Initialize :self _returnvalue_9 :InLayer -1.0 :InWidth (Variables|Default|GetPlayheadWidth) :InHeight (* (Variables|Default|GetCookSpawnVerticalPosition) -1.0) :ColorOff (LocalVariables|GetPlayheadColor))
  (Variables|Default|SetPlayhead _returnvalue_9)
  (CallFunction|UpdatePlayhead 0 0.0))

(fn AddSteps
  (bind _detailtilecolorfactor (Variables|Default|GetDetailTileColorFactor))
  (bind _ontilecolorfactor (Variables|Default|GetOnTileColorFactor))
  (for _array_element (Variables|/Script/FamJam.JamRecipe|GetSteps (Variables|Default|GetRecipe))
    (for _array_element_2 (.Chops (Utilities|Struct|BreakJamStep _array_element))
      (bind _returnvalue (Game|SpawnActorfromClass "/Game/Jam/Visualizer/BP_JamChopVisualizer.BP_JamChopVisualizer_C" (Math|Transform|MakeTransform (Math|Vector|MakeVector 0.0 (* (LocalVariables|GetMeasureStart) (+ (Variables|Default|GetMeasureHorizontalLength) (Variables|Default|GetMeasureHorizontalSpacing))) 0.0) "0, 0, 0" "1.000000,1.000000,1.000000") "Undefined" "MultiplyWithRoot" 0 0))
      (Transformation|AttachActorToActor _returnvalue (.CookLayerVIsualizer (Utilities|Struct|BreakF_JamCookLayerVisualizerContainer (Utilities|Array|Get(acopy) (.CookLayerVisualizers (Utilities|Struct|BreakF_JamCookVisualizerContainer (.Value (Utilities|Map|Find (Variables|Default|GetCookVisualizers) (.CookName (Utilities|Struct|BreakJamChop _array_element_2)))))) (- (.CookLayerIdx (Utilities|Struct|BreakJamChop _array_element_2)) 1)))) "None" "KeepRelative" "KeepRelative" "KeepRelative" true)
      (Default|Initialize _returnvalue (.MeasureStart (Utilities|Struct|BreakJamChop _array_element_2)) (.MeasureCount (Utilities|Struct|BreakJamChop _array_element_2)) (Variables|Default|GetMeasureHorizontalLength) (Variables|Default|GetMeasureHorizontalSpacing) (Variables|Default|GetMeasureVerticalLength) (Variables|Default|GetMeasureVerticalSpacing) (Math|Conversions|ToColor(LinearColor) (Utilities|Struct|MakeLinearColor (* (.r (Math|Conversions|ToLinearColor(Color) (.chopcolor (.Value (Utilities|Map|Find (.cooknametooverviewmap (Variables|Default|GetRecipeOverview)) (.CookName (Utilities|Struct|BreakJamChop _array_element_2))))))) _ontilecolorfactor) (* (.g (Math|Conversions|ToLinearColor(Color) (.chopcolor (.Value (Utilities|Map|Find (.cooknametooverviewmap (Variables|Default|GetRecipeOverview)) (.CookName (Utilities|Struct|BreakJamChop _array_element_2))))))) _ontilecolorfactor) (* (.b (Math|Conversions|ToLinearColor(Color) (.chopcolor (.Value (Utilities|Map|Find (.cooknametooverviewmap (Variables|Default|GetRecipeOverview)) (.CookName (Utilities|Struct|BreakJamChop _array_element_2))))))) _ontilecolorfactor) (.a (Math|Conversions|ToLinearColor(Color) (.chopcolor (.Value (Utilities|Map|Find (.cooknametooverviewmap (Variables|Default|GetRecipeOverview)) (.CookName (Utilities|Struct|BreakJamChop _array_element_2))))))))) (.chopcolor (.Value (Utilities|Map|Find (.cooknametooverviewmap (Variables|Default|GetRecipeOverview)) (.CookName (Utilities|Struct|BreakJamChop _array_element_2))))) (Math|Conversions|ToColor(LinearColor) (Utilities|Struct|MakeLinearColor (* (.r (Math|Conversions|ToLinearColor(Color) (.chopcolor (.Value (Utilities|Map|Find (.cooknametooverviewmap (Variables|Default|GetRecipeOverview)) (.CookName (Utilities|Struct|BreakJamChop _array_element_2))))))) _detailtilecolorfactor) (* (.g (Math|Conversions|ToLinearColor(Color) (.chopcolor (.Value (Utilities|Map|Find (.cooknametooverviewmap (Variables|Default|GetRecipeOverview)) (.CookName (Utilities|Struct|BreakJamChop _array_element_2))))))) _detailtilecolorfactor) (* (.b (Math|Conversions|ToLinearColor(Color) (.chopcolor (.Value (Utilities|Map|Find (.cooknametooverviewmap (Variables|Default|GetRecipeOverview)) (.CookName (Utilities|Struct|BreakJamChop _array_element_2))))))) _detailtilecolorfactor) (.a (Math|Conversions|ToLinearColor(Color) (.chopcolor (.Value (Utilities|Map|Find (.cooknametooverviewmap (Variables|Default|GetRecipeOverview)) (.CookName (Utilities|Struct|BreakJamChop _array_element_2)))))))))))
    (LocalVariables|SetMeasureStart (+ (LocalVariables|GetMeasureStart) (.MeasureLength (Utilities|Struct|BreakJamStep _array_element))))
    (bind _returnvalue_2 (Game|SpawnActorfromClass "/Game/Jam/Visualizer/BP_JamRecipeDivider.BP_JamRecipeDivider_C" (Math|Transform|MakeTransform (Math|Vector|MakeVector 0.0 (+ (* (LocalVariables|GetMeasureStart) (Variables|Default|GetMeasureHorizontalLength)) (* (- (LocalVariables|GetMeasureStart) 0.75) (Variables|Default|GetMeasureHorizontalSpacing))) 0.0) "0, 0, 0" "1.000000,1.000000,1.000000") "Undefined" "MultiplyWithRoot" 0 0))
    (Transformation|AttachActorToActor _returnvalue_2 self "None" "KeepRelative" "KeepRelative" "KeepRelative" true)
    (Default|Initialize :self _returnvalue_2 :InLayer 1.5 :InWidth (/ (Variables|Default|GetMeasureHorizontalSpacing) 2.0) :InHeight (* (Variables|Default|GetCookSpawnVerticalPosition) -1.0) :ColorOff (LocalVariables|GetStepDividerColor))))

(fn Update
  (params (StepIdx :type Integer) (MeasuresRemaining :type Float%20%28double-precision%29))
  (CallFunction|UpdatePlayhead StepIdx (- (.measurelength (Utilities|Array|Get(acopy) (Variables|/Script/FamJam.JamRecipe|GetSteps (Variables|Default|GetRecipe)) StepIdx)) MeasuresRemaining))
  (CallFunction|UpdateTiles))

(fn UpdatePlayhead
  (params (StepIdx :type Integer) (MeasuresLocation :type Float%20%28double-precision%29))
  (for _index (range 0 (- StepIdx 1))
    (LocalVariables|SetPreviousMeasuresCount (+ (LocalVariables|GetPreviousMeasuresCount) (.measurelength (Utilities|Array|Get(acopy) (Variables|/Script/FamJam.JamRecipe|GetSteps (Variables|Default|GetRecipe)) _index)))))
  (Transformation|SetActorRelativeLocation (Variables|Default|GetPlayhead) (Math|Vector|MakeVector 0.0 (+ (* (+ MeasuresLocation (LocalVariables|GetPreviousMeasuresCount)) (Variables|Default|GetMeasureHorizontalLength)) (* (Math|Float|Floor (+ MeasuresLocation (LocalVariables|GetPreviousMeasuresCount))) (Variables|Default|GetMeasureHorizontalSpacing)) (* (Variables|Default|GetPlayheadWidth) -1.0)) 0.0)))

(fn UpdateTiles)