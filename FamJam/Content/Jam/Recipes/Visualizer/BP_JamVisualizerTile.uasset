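; BP_JamVisualizerTile is a single colored box tile for the Jam recipe visualizer.
; Initialize scales the Tile mesh from width, height and LayerDepth, assuming a 100-unit base mesh, and steps it along X by layer index.
; Half-size Y and Z offsets put the actor origin at a corner, with the tile extending toward +Y and -Z.
; The given color feeds the material's "color" vector parameter.
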(event EventBeginPlay)

(event Collision|EventActorBeginOverlap
  (params (OtherActor :type Actor%20Object%20Reference)))

(event EventTick
  (params (DeltaSeconds :type Float%20%28single-precision%29)))

(fn ConstructionScript)

(fn Initialize
  (params (InLayer :type Integer) (InWidth :type Float%20%28double-precision%29) (InHeight :type Float%20%28double-precision%29) (Color :type Color%20Structure))
  (bind _returnvalue (Math|Conversions|ToLinearColor(Color) Color))
  (bind _tile (Variables|Default|GetTile))
  (bind (_r _g _b) (Utilities|Struct|BreakLinearColor _returnvalue))
  (Transformation|SetWorldScale3D _tile (Math|Vector|MakeVector (/ (Variables|Default|GetLayerDepth) 1e+02) (/ InWidth 1e+02) (/ InHeight 1e+02)))
  (Transformation|SetRelativeLocation _tile (Math|Vector|MakeVector (* InLayer (Variables|Default|GetLayerDepth)) (/ InWidth 2.0) (/ InHeight -2.0)) false false)
  (Rendering|Material|SetVectorParameterValueonMaterials _tile "color" (Math|Vector|MakeVector _r _g _b)))