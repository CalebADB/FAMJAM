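; Visualizes a jam chunk as a row of measure segments along the Y axis, built from child visualizer actors.
; Initialize spawns and attaches BP_JamChunkMeasureVisualizer segments with BP_JamChunkEdgeVisualizer dividers and end caps, using the given sizes and colors.
; Fractional starts and lengths produce partial-width first and last measures, as a loop consumes the remaining measure count.
; When destroyed, it destroys its attached actors.
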(event EventBeginPlay)

(event Collision|EventActorBeginOverlap
  (params (OtherActor :type Actor%20Object%20Reference)))

(event EventTick
  (params (DeltaSeconds :type Float%20%28single-precision%29)))

(event EventDestroyed
  (bind _self self)
  (bind _outactors (Actor|GetAttachedActors _self true false))
  (if (not (== (Utilities|Array|Length _outactors) 0)) :!label _label
    (Actor|DestroyActor (Utilities|Array|Get(acopy) _outactors))
    (goto _label)))

(fn ConstructionScript)

(fn Initialize
  (params (MeasureStart :type Float%20%28double-precision%29) (TotalMeasureCount :type Float%20%28double-precision%29) (MeasureWidth :type Float%20%28double-precision%29) (MeasureWidthSpacing :type Float%20%28double-precision%29) (MeasureHeight :type Float%20%28double-precision%29) (MeasureHeightSpacing :type Float%20%28double-precision%29) (MeasureColorOn :type Color%20Structure) (MeasureColorOff :type Color%20Structure) (MeasureDetailColor :type Color%20Structure))
  (bind (_remainder _returnvalue) (Math|Float|Division(WholeandRemainder) MeasureStart 1.0))
  (bind _returnvalue_2 (+ MeasureStart TotalMeasureCount))
  (Variables|Default|SetRemainingMeasureCount TotalMeasureCount)
  (Variables|Default|SetNextMeasureLocation _returnvalue)
  (bind _returnvalue_3 (Game|SpawnActorfromClass "/Game/Jam/Recipes/Visualizer/BP_JamChunkEdgeVisualizer.BP_JamChunkEdgeVisualizer_C" (Math|Transform|MakeTransform (Math|Vector|MakeVector 0.0 (+ (* (+ _remainder (Variables|Default|GetNextMeasureLocation)) MeasureWidth) (* (Variables|Default|GetNextMeasureLocation) MeasureWidthSpacing)) 0.0) "0, 0, 0" "1.000000,1.000000,1.000000") "Undefined" "MultiplyWithRoot" 0 0))
  (Transformation|AttachActorToActor _returnvalue_3 self "None" "KeepRelative" "KeepRelative" "KeepRelative" true)
  (Default|Initialize :self _returnvalue_3 :InWidth (/ MeasureWidthSpacing 2.0) :InHeight (+ MeasureHeight MeasureHeightSpacing) :ColorOff MeasureDetailColor)
  (if (> _remainder 0.0)
    (bind _returnvalue_4 (Game|SpawnActorfromClass "/Game/Jam/Recipes/Visualizer/BP_JamChunkMeasureVisualizer.BP_JamChunkMeasureVisualizer_C" (Math|Transform|MakeTransform (Math|Vector|MakeVector 0.0 (+ (* (+ _remainder (Variables|Default|GetNextMeasureLocation)) MeasureWidth) (* (Variables|Default|GetNextMeasureLocation) MeasureWidthSpacing)) (/ MeasureHeightSpacing -2.0)) "0, 0, 0" "1.000000,1.000000,1.000000") "Undefined" "MultiplyWithRoot" 0 0))
    (Transformation|AttachActorToActor _returnvalue_4 self "None" "KeepRelative" "KeepRelative" "KeepRelative" true)
    (Default|Initialize _returnvalue_4 (Math|Conversions|ToFloat(Integer) (Class|KismetSystemLibrary|MakeLiteralInteger 1)) (* (Math|Float|Clamp(Float) (Variables|Default|GetRemainingMeasureCount) 0.0 (- 1.0 _remainder)) MeasureWidth) MeasureHeight MeasureColorOn MeasureColorOff)
    (Variables|Default|SetLastMeasureWidth (Math|Float|Clamp(Float) (Variables|Default|GetRemainingMeasureCount) 0.0 (- 1.0 _remainder)))
    (Variables|Default|SetRemainingMeasureCount (- (Variables|Default|GetRemainingMeasureCount) (Math|Float|Clamp(Float) (Variables|Default|GetRemainingMeasureCount) 0.0 (- 1.0 _remainder))))
    (bind _result (Math|Integer|IncrementInt (Variables|Default|GetNextMeasureLocation) :!label _label)
      (:%20%20
        (if (> (Variables|Default|GetRemainingMeasureCount) 0.0)
          (bind _returnvalue_5 (Game|SpawnActorfromClass "/Game/Jam/Recipes/Visualizer/BP_JamChunkEdgeVisualizer.BP_JamChunkEdgeVisualizer_C" (Math|Transform|MakeTransform (Math|Vector|MakeVector 0.0 (+ (* MeasureWidth _result) (* MeasureWidthSpacing (- _result 1))) (/ MeasureHeight -2.0)) "0, 0, 0" "1.000000,1.000000,1.000000") "Undefined" "MultiplyWithRoot" 0 0))
          (Transformation|AttachActorToActor _returnvalue_5 self "None" "KeepRelative" "KeepRelative" "KeepRelative" true)
          (Default|Initialize :self _returnvalue_5 :InWidth MeasureWidthSpacing :InHeight MeasureHeightSpacing :ColorOff MeasureDetailColor)
          (bind _returnvalue_6 (Game|SpawnActorfromClass "/Game/Jam/Recipes/Visualizer/BP_JamChunkMeasureVisualizer.BP_JamChunkMeasureVisualizer_C" (Math|Transform|MakeTransform (Math|Vector|MakeVector 0.0 (+ (* (Variables|Default|GetNextMeasureLocation) MeasureWidth) (* (Variables|Default|GetNextMeasureLocation) MeasureWidthSpacing)) (/ MeasureHeightSpacing -2.0)) "0, 0, 0" "1.000000,1.000000,1.000000") "Undefined" "MultiplyWithRoot" 0 0 :!label _label_2))
          (Transformation|AttachActorToActor _returnvalue_6 self "None" "KeepRelative" "KeepRelative" "KeepRelative" true)
          (Default|Initialize _returnvalue_6 (Math|Conversions|ToFloat(Integer) (Class|KismetSystemLibrary|MakeLiteralInteger 1)) (* MeasureWidth (Math|Float|Clamp(Float) (Variables|Default|GetRemainingMeasureCount))) MeasureHeight MeasureColorOn MeasureColorOff)
          (Variables|Default|SetLastMeasureWidth (* MeasureWidth (Math|Float|Clamp(Float) (Variables|Default|GetRemainingMeasureCount))))
          (Variables|Default|SetRemainingMeasureCount (- (Variables|Default|GetRemainingMeasureCount) (Math|Float|Clamp(Float) (Variables|Default|GetRemainingMeasureCount))))
          (goto _label)
          (else
            _))))
    (else
      (Variables|Default|SetNextMeasureLocation (Math|Float|Round MeasureStart))
      (if (> (Variables|Default|GetRemainingMeasureCount) 0.0)
        (goto _label_2)
        (else
          _))))
  (bind _returnvalue_7 (Game|SpawnActorfromClass "/Game/Jam/Recipes/Visualizer/BP_JamChunkEdgeVisualizer.BP_JamChunkEdgeVisualizer_C" (Math|Transform|MakeTransform (Math|Vector|MakeVector 0.0 (- (+ (* MeasureWidth _returnvalue_2) (* MeasureWidthSpacing (- (Math|Float|Ceil _returnvalue_2) 1))) (/ MeasureWidthSpacing 2.0)) 0.0) "0, 0, 0" "1.000000,1.000000,1.000000") "Undefined" "MultiplyWithRoot" 0 0))
  (Transformation|AttachActorToActor _returnvalue_7 self "None" "KeepRelative" "KeepRelative" "KeepRelative" true)
  (Default|Initialize :self _returnvalue_7 :InWidth (/ MeasureWidthSpacing 2.0) :InHeight (+ MeasureHeight MeasureHeightSpacing) :ColorOff MeasureDetailColor))