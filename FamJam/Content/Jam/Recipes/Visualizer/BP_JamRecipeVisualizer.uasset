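; Actor that draws a jam recipe, looked up by row name on BeginPlay, as a timeline of measures, printing an error if none is found.
; Initialize builds vertically stacked cook panels from the recipe overview, each holding alternately colored layer rows, and stores them in a map by cook name.
; AddStep spawns a chunk visualizer per chop, offset by step start measure and attached to its cook's layer.
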(event EventBeginPlay
  (bind _reciperowname (Variables|Default|GetRecipeRowName))
  (bind _returnvalue (Class|JamRecipeLibrarian|GetRecipe (Variables|Default|GetJamRecipeLibrarian) _reciperowname))
  (if (!= _returnvalue 0)
    (bind _output_get (Variables|Default|SetRecipe _returnvalue))
    (bind _returnvalue_2 (Class|JamRecipe|GetOverview _output_get))
    (CallFunction|Initialize _returnvalue_2)
    (for _array_element (Variables|/Script/FamJam.JamRecipe|GetSteps _output_get)
      (CallFunction|AddStep _array_element))
    (else
      (Development|PrintString (Utilities|String|Append "Could not find RowName: " (Utilities|String|ToString(Name) _reciperowname)) true true "(R=1.000000,G=0.366009,B=0.000000,A=1.000000)" 1e+01))))

(event Collision|EventActorBeginOverlap
  (params (OtherActor :type Actor%20Object%20Reference)))

(event EventTick
  (params (DeltaSeconds :type Float%20%28single-precision%29)))

(fn ConstructionScript)

(fn AddStep
  (params (Step :type Jam%20Step%20Structure))
  (bind (_measurestart _measurescount _specialactionkeytoparamsmap _chops) (Utilities|Struct|BreakJamStep Step))
  (for _array_element _chops
    (bind _returnvalue (Game|SpawnActorfromClass "/Game/Jam/Recipes/Visualizer/BP_JamChunkVisualizer.BP_JamChunkVisualizer_C" (Math|Transform|MakeTransform (Math|Vector|MakeVector 0.0 (* _measurestart (+ (Variables|Default|GetMeasureHorizontalLength) (Variables|Default|GetMeasureHorizontalSpacing))) 0.0) "0, 0, 0" "1.000000,1.000000,1.000000") "Undefined" "MultiplyWithRoot" 0 0))
    (Transformation|AttachActorToActor _returnvalue (.CookLayerVIsualizer (Utilities|Struct|BreakF_JamCookLayerVisualizerContainer (Utilities|Array|Get(acopy) (.CookLayers (Utilities|Struct|BreakF_JamCookVisualizerContainer (.Value (Utilities|Map|Find (Variables|Default|GetCookVisualizers) (.CookName (Utilities|Struct|BreakJamChop _array_element)))))) (- (.CookLayer (Utilities|Struct|BreakJamChop _array_element)) 1)))) "None" "KeepRelative" "KeepRelative" "KeepRelative" true)
    (Default|Initialize _returnvalue (.MeasureStart (Utilities|Struct|BreakJamChop _array_element)) (.MeasureCount (Utilities|Struct|BreakJamChop _array_element)) (Variables|Default|GetMeasureHorizontalLength) (Variables|Default|GetMeasureHorizontalSpacing) (Variables|Default|GetMeasureVerticalLength))))

(fn Initialize
  (params (RecipeOverview :type Jam%20Recipe%20Overview%20Structure))
  (bind (_lastmeasure _volumeratiomax _cooknametolayercountmap _cooknametodebugcolormap) (Utilities|Struct|BreakJamRecipeOverview RecipeOverview))
  (bind _cookvisualizers (Variables|Default|GetCookVisualizers))
  (bind _cooklayerverticallength (Variables|Default|GetCookLayerVerticalLength))
  (bind _measurehorizontalspacing (Variables|Default|GetMeasureHorizontalSpacing))
  (bind _measurehorizontallength (Variables|Default|GetMeasureHorizontalLength))
  (bind _returnvalue (- _lastmeasure 1.0))
  (bind _returnvalue_2 (* _lastmeasure _measurehorizontallength))
  (bind _returnvalue_3 (* _returnvalue _measurehorizontalspacing))
  (bind _returnvalue_4 (+ _returnvalue_2 _returnvalue_3))
  (Variables|Default|SetCookSpawnVerticalPosition (/ (Variables|Default|GetCookVerticalSpacing) -2.0))
  (bind _keys (Utilities|Map|Keys _cooknametolayercountmap))
  (for _array_element _keys
    (bind _returnvalue_5 (Game|SpawnActorfromClass "/Game/Jam/Recipes/Visualizer/BP_JamCookVisualizer.BP_JamCookVisualizer_C" (Math|Transform|MakeTransform (Math|Vector|MakeVector 0.0 0.0 (Variables|Default|GetCookSpawnVerticalPosition)) "0, 0, 0" "1.000000,1.000000,1.000000") "Undefined" "MultiplyWithRoot" 0 0))
    (Transformation|AttachActorToActor _returnvalue_5 self "None" "KeepRelative" "KeepRelative" "KeepRelative" true)
    (Utilities|Map|Add _cookvisualizers _array_element (Utilities|Struct|MakeF_JamCookVisualizerContainer _returnvalue_5))
    (Default|Initialize _returnvalue_5 3 _returnvalue_4 (* (+ (Variables|Default|GetCookLayerVerticalSpacing) (Variables|Default|GetCookLayerVerticalLength)) (.Value (Utilities|Map|Find _cooknametolayercountmap _array_element))) (.Value (Utilities|Map|Find _cooknametodebugcolormap _array_element)))
    (Variables|Default|SetCookLayerSpawnVerticalPosition (/ (Variables|Default|GetCookLayerVerticalSpacing) -2.0))
    (for _index (range 1 (.Value (Utilities|Map|Find _cooknametolayercountmap _array_element)))
      (bind _returnvalue_6 (Game|SpawnActorfromClass "/Game/Jam/Recipes/Visualizer/BP_JamCookLayerVisualizer.BP_JamCookLayerVisualizer_C" (Math|Transform|MakeTransform (Math|Vector|MakeVector 0.0 0.0 (Variables|Default|GetCookLayerSpawnVerticalPosition)) "0, 0, 0" "1.000000,1.000000,1.000000") "Undefined" "MultiplyWithRoot" 0 0))
      (Transformation|AttachActorToActor _returnvalue_6 (.CookVisualizer (Utilities|Struct|BreakF_JamCookVisualizerContainer (.Value (Utilities|Map|Find _cookvisualizers _array_element)))) "None" "KeepRelative" "KeepRelative" "KeepRelative" true)
      (Utilities|Array|Add (Variables|Default|GetCookLayerVisualizers) (Utilities|Struct|MakeF_JamCookLayerVisualizerContainer _returnvalue_6))
      (if (Variables|Default|GetbShouldUseCookLayerColorA)
        (Default|Initialize _returnvalue_6 2 _returnvalue_4 _cooklayerverticallength (Variables|Default|GetCookLayerColorA))
        (Variables|Default|SetbShouldUseCookLayerColorA false)
        (else
          (Default|Initialize _returnvalue_6 2 _returnvalue_4 _cooklayerverticallength (Variables|Default|GetCookLayerColorB))
          (Variables|Default|SetbShouldUseCookLayerColorA true)))
      (Variables|Default|SetCookLayerSpawnVerticalPosition (- (- (Variables|Default|GetCookLayerSpawnVerticalPosition) (Variables|Default|GetCookLayerVerticalLength)) (Variables|Default|GetCookLayerVerticalSpacing))))
    (Variables|Default|SetCookSpawnVerticalPosition (- (- (Variables|Default|GetCookSpawnVerticalPosition) (* (+ (Variables|Default|GetCookLayerVerticalSpacing) (Variables|Default|GetCookLayerVerticalLength)) (.Value (Utilities|Map|Find _cooknametolayercountmap _array_element)))) (Variables|Default|GetCookVerticalSpacing)))
    (bind _output_get (Variables|Default|SetCookVisualizer (.CookVisualizer (Utilities|Struct|BreakF_JamCookVisualizerContainer (.Value (Utilities|Map|Find _cookvisualizers _array_element))))))
    (Utilities|Map|Remove _cookvisualizers _array_element)
    (Utilities|Map|Add _cookvisualizers _array_element (Utilities|Struct|MakeF_JamCookVisualizerContainer _output_get (Variables|Default|GetCookLayerVisualizers)))
    (Utilities|Array|Clear (Variables|Default|GetCookLayerVisualizers))))